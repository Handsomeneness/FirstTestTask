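; BP_Valve is a grabbable valve, built from torus shapes and an arrow, that rotates around yaw.
; The left grab input calls an attach on ShapeTorus1 with keep-relative rules and no parent specified.
; Every tick, the world Y offset from ShapeTorus1 to Arrow is added to ShapeTorus's yaw, which is clamped to one full turn, without delta-time scaling.
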(event Input|EnhancedActionEvents|EnhancedInputActionIA_Grab_Left
  (params (ActionValue :type Float%20%28double-precision%29) (ElapsedSeconds :type Float%20%28double-precision%29) (TriggeredSeconds :type Float%20%28double-precision%29) (InputAction :type Input%20Action%20Object%20Reference :default "/Game/VRTemplate/Input/Actions/IA_Grab_Left.IA_Grab_Left"))
  (:Started
    (Transformation|AttachComponentToComponent (Variables|Default|GetShape_Torus1) 0 "None" "KeepRelative" "KeepRelative" "KeepRelative" true)))

(event EventTick
  (params (DeltaSeconds :type Float%20%28single-precision%29))
  (bind _shape_torus (Variables|Default|GetShape_Torus))
  (bind _returnvalue (Transformation|GetWorldRotation _shape_torus))
  (Transformation|SetWorldRotation _shape_torus (Math|Rotator|MakeRotator (.roll _returnvalue) (.pitch _returnvalue) (Math|Float|Clamp(Float) (+ (.y (- (Transformation|GetWorldLocation (Variables|Default|GetArrow)) (Transformation|GetWorldLocation (Variables|Default|GetShape_Torus1)))) (.yaw _returnvalue)) 0.0 3.6e+02)) false false))

(fn ConstructionScript)