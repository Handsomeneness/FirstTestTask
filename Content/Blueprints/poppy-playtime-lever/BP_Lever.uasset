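; BP_Lever is a lever actor whose roll follows the vertical position of a Cube component.
; The left grab input attaches the Cube with keep-relative rules, with no parent shown.
; Every tick, the height difference between an Arrow and the Cube is added to the Lever's world roll, clamped to a symmetric range.
; No release handling is present.
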(event Input|EnhancedActionEvents|EnhancedInputActionIA_Grab_Left
  (params (ActionValue :type Float%20%28double-precision%29) (ElapsedSeconds :type Float%20%28double-precision%29) (TriggeredSeconds :type Float%20%28double-precision%29) (InputAction :type Input%20Action%20Object%20Reference :default "/Game/VRTemplate/Input/Actions/IA_Grab_Left.IA_Grab_Left"))
  (:Started
    (Transformation|AttachComponentToComponent (Variables|Default|GetCube) 0 "None" "KeepRelative" "KeepRelative" "KeepRelative" true)))

(event EventTick
  (params (DeltaSeconds :type Float%20%28single-precision%29))
  (bind _lever (Variables|Default|GetLever))
  (bind _returnvalue (Transformation|GetWorldRotation _lever))
  (Transformation|SetWorldRotation _lever (Math|Rotator|MakeRotator (Math|Float|Clamp(Float) (+ (.z (- (Transformation|GetWorldLocation (Variables|Default|GetArrow)) (Transformation|GetWorldLocation (Variables|Default|GetCube)))) (.roll _returnvalue)) -6e+01 6e+01) (.pitch _returnvalue) (.yaw _returnvalue)) false false))

(fn ConstructionScript)